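; BP_SunDay is the sun actor that runs a looping night/day cycle, starting at night.
; Two timelines alternate, each rotating the actor a half turn, snapping it back, swapping the face material and notifying the Game Instance of phase changes.
; KillAI_SpeedUpRate raises the day timeline's play rate until a phase end resets it.
; Tick keeps the sphere facing the player.
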(event `self.ReceiveTick`
  (params (DeltaSeconds :type "Float (single-precision)"))
  (bind _sphere (`self.Sphere`))
  (`SceneComponent.K2_SetWorldRotation` _sphere (`KismetMathLibrary.FindLookAtRotation` (`SceneComponent.K2_GetComponentLocation` _sphere) (`self.K2_GetActorLocation` (`GameplayStatics.GetPlayerCharacter` 0))) false false))

(event `self.ReceiveBeginPlay`
  (bind _output_get (set `self.InitPlayRate` (`TimelineComponent.GetPlayRate` (`self.SpeedSunTimeline`))))
  (set `self.ActualPlayRate` _output_get)
  (`self.StartNight`))

(event `KillAI_SpeedUpRate`
  (bind _speedsuntimeline (`self.SpeedSunTimeline`))
  (`TimelineComponent.SetPlayRate` _speedsuntimeline (+ (`self.ActualPlayRate`) 0.5))
  (set `self.ActualPlayRate` (`TimelineComponent.GetPlayRate` _speedsuntimeline)))

(event `StartTimerDay`
  (bind _initrotation (`self.InitRotation`))
  (`/Game/Root/Utils/MyGI.ED_StartDay` (`/Game/Root/Utils/Utils.GetGI`))
  (set `self.InitRotation` (`self.K2_GetActorRotation`))
  (`PrimitiveComponent.SetMaterial` (`self.Face`) 0 "/Game/Root/IA/Ennemy_02/Baby_01.Baby_01")
  (bind (_direction _newtrack_0) (`Timeline|SpeedSunTimeline` :!via `PlayFromStart`)
    (:`Update`
      (`self.K2_SetActorRotation` (`KismetMathLibrary.RLerp` _initrotation (`KismetMathLibrary.ComposeRotators` _initrotation (`KismetMathLibrary.RotatorFromAxisAndAngle` (1.0 0.0 0.0) 180.0)) _newtrack_0)))
    (:`Finished`
      (`self.K2_SetActorRotation` (`self.InitRotation`))
      (`KismetSystemLibrary.PrintString` "EndDay/StartNight")
      (`self.StartNight`)
      (`self.ResetPlayRate`)
      (`/Game/Root/Utils/MyGI.ED_StartNight` (`/Game/Root/Utils/Utils.GetGI`)))))

(event `StartNight`
  (bind _initrotation (`self.InitRotation`))
  (`/Game/Root/Utils/MyGI.ED_StartNight` (`/Game/Root/Utils/Utils.GetGI`))
  (set `self.InitRotation` (`self.K2_GetActorRotation`))
  (`PrimitiveComponent.SetMaterial` (`self.Face`) 0 "/Game/Root/IA/Baby/Happy_Ba.Happy_Ba")
  (bind (_direction _newtrack_0) (`Timeline|SpeedNightTimeline` :!via `PlayFromStart`)
    (:`Update`
      (`self.K2_SetActorRotation` (`KismetMathLibrary.RLerp` _initrotation (`KismetMathLibrary.ComposeRotators` _initrotation (`KismetMathLibrary.RotatorFromAxisAndAngle` (1.0 0.0 0.0) 180.0)) _newtrack_0)))
    (:`Finished`
      (`self.K2_SetActorRotation` (`self.InitRotation`))
      (`self.StartTimerDay`)
      (`KismetSystemLibrary.PrintString` "EndNight/StartDay")
      (`self.ResetPlayRate`))))

(event `ResetPlayRate`
  (`TimelineComponent.SetPlayRate` (`self.SpeedSunTimeline`) 1.0)
  (set `self.ActualPlayRate` 1.0))

(fn `UserConstructionScript`
  (bind _returnvalue (`PrimitiveComponent.CreateDynamicMaterialInstance` (`self.Sphere`) 0 "/Engine/BasicShapes/BasicShapeMaterial.BasicShapeMaterial" "None"))
  (set `self.DynMat` _returnvalue))