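; BP_Collectibles is a pickup that gives the player a bonus of its Type on overlap when CanPickup is set, then destroys itself.
; A looping timer spins the Scene component and uses sine-driven lerps to pulse its scale and bob its height.
; It binds to the GameInstance day/night events to count days lived, despawning at nightfall once the limit is reached, skipping the first night if spawned by day.
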(event `CustomEvent_0`
  (if (`self.SpawnDuringTheDay`)
    (set `self.SpawnDuringTheDay` false)
    (elif (>= (`self.numberOfDay`) (`self.numberOfDayBeforeDespawn`))
      (`self.K2_DestroyActor`))))

(event `self.ReceiveBeginPlay`
  (bind _output_get (set `self.SpawnDuringTheDay` (`/Game/Root/Utils/MyGI.IsDay?` (`/Game/Root/Utils/Utils.GetGI`))))
  (if _output_get
    (`/Engine/EditorBlueprintResources/StandardMacros.IncrementInt` (`self.numberOfDay`)
      (:`  `
        _)))
  (`KismetSystemLibrary.K2_SetTimerDelegate` (delegate `CustomEvent`) 0.05 true)
  (set `self.initScale` (`SceneComponent.RelativeScale3D` (`self.Scene`)))
  (set `self.InitLocaiton` (`SceneComponent.RelativeLocation` (`self.Scene`)))
  (add `/Game/Root/Utils/MyGI.ED_StartNight` (`/Game/Root/Utils/Utils.GetGI`) (delegate `CustomEvent_0`))
  (add `/Game/Root/Utils/MyGI.ED_StartDay` (`/Game/Root/Utils/Utils.GetGI`) (delegate `CustomEvent_1`)))

(event `CustomEvent_1`
  (if (not (`self.SpawnDuringTheDay`))
    (`/Engine/EditorBlueprintResources/StandardMacros.IncrementInt` (`self.numberOfDay`))))

(event `CustomEvent`
  (`SceneComponent.K2_AddRelativeRotation` (`self.Scene`) (`KismetMathLibrary.RotatorFromAxisAndAngle` (0.0 0.0 1.0) (`self.RotationSpeed`)) false false)
  (set `self.elapseTime` (+ (`self.elapseTime`) (* (`GameplayStatics.GetWorldDeltaSeconds`) (`self.AnimSpeed`))))
  (`self.ScaleOverTime` (`self.elapseTime`))
  (`self.NewFunction` (`self.elapseTime`)))

(event `self.Box.OnComponentBeginOverlap`
  (params (OverlappedComponent :type "PrimitiveComponent Object Reference") (OtherActor :type "Actor Object Reference") (OtherComp :type "PrimitiveComponent Object Reference") (OtherBodyIndex :type Integer) (bFromSweep :type Boolean) (SweepResult :type "HitResult Structure (by ref)"))
  (if (== OtherActor (`/Game/Root/Utils/Utils.GetMyPlayer`))
    (if (`self.CanPickup`)
      (`self.GiveBonus`)
      (`self.K2_DestroyActor`))))

(fn `GiveBonus`
  (`/Game/FirstPerson/Blueprints/BP_FirstPersonCharacter.GetBonus` (`/Game/Root/Utils/Utils.GetMyPlayer`) (`self.Type`)))

(fn `NewFunction`
  (params (A :type "Float (double-precision)"))
  (bind (_initlocaiton_x _initlocaiton_y _initlocaiton_z) (`KismetMathLibrary.BreakVector` (`self.InitLocaiton`)))
  (`SceneComponent.K2_SetRelativeLocation` (`self.Scene`) (`KismetMathLibrary.VLerp` (`KismetMathLibrary.MakeVector` 0.0 0.0 (+ _initlocaiton_z 15.0)) (`KismetMathLibrary.MakeVector` 0.0 0.0 (- _initlocaiton_z 15.0)) (`KismetMathLibrary.Sin` A)) false false))

(fn `ScaleOverTime`
  (params (A :type "Float (double-precision)"))
  (`SceneComponent.SetRelativeScale3D` (`self.Scene`) (`KismetMathLibrary.VLerp` (* (`self.initScale`) 1.3) (* (`self.initScale`) 1.0) (`KismetMathLibrary.Sin` A))))

(fn `UserConstructionScript`)