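; BP_Shotgun is the player's shotgun actor, handling procedural shoot, reload and melee animation with reload sounds.
; Timelines lerp the actor's relative location and rotation for recoil, reload turn and melee thrust, stopping competing timelines when shooting or meleeing.
; Shooting also spawns a particle effect at the Scene component and, unless Akimbo, chains into a reload when the recoil finishes.
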(event `ShootAnim`
  (params (Akimbo :type Boolean))
  (bind _scene (`self.Scene`))
  (set `self.Akimbo` Akimbo)
  (`|ExecutionSequence`
    (:`then_0`
      (bind (_direction _reload) (`Timeline|Reload` :!via `Stop` :!label _label)
        (:`Update`
          (`self.K2_SetActorRelativeRotation` (`KismetMathLibrary.RLerp` (struct) (`self.ReloadRotation`) _reload)))))
    (:`then_1`
      (bind (_direction_2 _meleerotation _meleeforward) (`Timeline|Melee` :!via `Stop` :!label _label_2)
        (:`Update`
          (`self.K2_SetActorRelativeRotation` (`KismetMathLibrary.RLerp` (struct) (`self.MeeleRotation`) _meleerotation))
          (`self.K2_SetActorRelativeLocation` (`KismetMathLibrary.VLerp` (0.0 0.0 0.0) (`self.MeleeForward`) _meleeforward)))))
    (:`then_2`
      (bind (_direction_3 _back _roll) (`Timeline|Shoot` :!via `PlayFromStart` :!label _label_3)
        (:`Update`
          (`self.K2_SetActorRelativeLocation` (`KismetMathLibrary.VLerp` (0.0 0.0 0.0) (`self.PushBack`) _back))
          (`self.K2_SetActorRelativeRotation` (`KismetMathLibrary.RLerp` (struct) (`self.PushTurn`) _roll)))
        (:`Finished`
          (if (not (`self.Akimbo`))
            (`GameplayStatics.PlaySound2D` "/Game/Root/Sound_Design/SFX/Player/P_Shotgun_Reload.P_Shotgun_Reload" 1.0 1.0 0.0 null null)
            (goto _label :!via `PlayFromStart`)))))
    (:`then_3`
      (`NiagaraFunctionLibrary.SpawnSystemAtLocation` "/Game/CORE/ART/VFX/Player/PS_Bonk.PS_Bonk" (`SceneComponent.K2_GetComponentLocation` _scene) (`SceneComponent.K2_GetComponentRotation` _scene)))))

(event `ReloadAnim`
  (`GameplayStatics.PlaySound2D` "/Game/Root/Sound_Design/SFX/Player/P_DoubleShotgun_Reload.P_DoubleShotgun_Reload" 1.0 1.0 0.0 null null)
  (goto _label :!via `PlayFromStart`))

(event `MeleeAnim`
  (`|ExecutionSequence`
    (:`then_0`
      (goto _label_3 :!via `Stop`))
    (:`then_1`
      (goto _label :!via `Stop`))
    (:`then_2`
      (goto _label_2 :!via `PlayFromStart`))))

(fn `UserConstructionScript`)