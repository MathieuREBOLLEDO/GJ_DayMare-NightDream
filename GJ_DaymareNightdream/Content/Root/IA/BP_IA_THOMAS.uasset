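; Thomas train enemy derived from BP_IA that explodes both when it attacks and when it dies.
; Swaps face materials on night/day events, animates its chimney scale and spins its wheels while moving.
; A one-shot Explosion scales the body via timeline, launches its parts as physics debris, then sphere-traces forward to damage the player and other AI.
; It then calls parent death logic and destroys itself after a delay.
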(event `ChangeFaceNight`
  (`PrimitiveComponent.SetMaterial` (`self.Face`) 0 "/Game/Root/IA/Ennemy_02/Thomas_Face_Happy.Thomas_Face_Happy"))

(event `ChangeFaceDay`
  (`PrimitiveComponent.SetMaterial` (`self.Face`) 0 "/Game/Root/IA/Ennemy_02/Thomas_Face_Happy1.Thomas_Face_Happy1"))

(event `self.ReceiveBeginPlay`
  (bind (_initscale_x _initscale_y) (`KismetMathLibrary.BreakVector` (`self.InitScale`)))
  (`parent.ReceiveBeginPlay`)
  (`|ExecutionSequence`
    (:`then_0`
      (add `/Game/Root/Utils/MyGI.ED_StartNight` (`/Game/Root/Utils/Utils.GetGI`) (delegate `ChangeFaceNight`))
      (add `/Game/Root/Utils/MyGI.ED_StartDay` (`/Game/Root/Utils/Utils.GetGI`) (delegate `ChangeFaceDay`)))
    (:`then_1`
      (set `self.InitScale` (`SceneComponent.K2_GetComponentScale` (`self.chemi`)))
      (`TimelineComponent.SetPlayRate` (`self.ChemineScale`) 1.5)
      (bind (_direction _newtrack_0) (`Timeline|ChemineScale` :!via `PlayFromStart`)
        (:`Update`
          (bind _returnvalue (`KismetMathLibrary.Lerp` _initscale_x (/ _initscale_x 1.5) _newtrack_0))
          (`SceneComponent.SetWorldScale3D` (`self.chemi`) (`KismetMathLibrary.MakeVector` _returnvalue _returnvalue (`KismetMathLibrary.Lerp` _initscale_y (/ _initscale_y 1.2) _newtrack_0))))))))

(event `self.ReceiveTick`
  (params (DeltaSeconds :type "Float (single-precision)"))
  (bind _array (`|MakeArray` (`self.rou`) (`self.rou1`) (`self.rou2`) (`self.rou6`) (`self.rou7`) (`self.rou8`)))
  (`parent.ReceiveTick` DeltaSeconds)
  (if (`self.OnMovement?`)
    (for (_array_element _array_index) _array
      (`KismetArrayLibrary.Array_Set` (`self.WheelsRotInit`) _array_index (`SceneComponent.RelativeRotation` _array_element)))
    (for (_array_element_2 _array_index_2) _array
      (`SceneComponent.K2_SetRelativeRotation` _array_element_2 (`KismetMathLibrary.ComposeRotators` (`|GetArrayItem` (`self.WheelsRotInit`) _array_index_2) (`KismetMathLibrary.RotatorFromAxisAndAngle` (1.0 0.0 0.0) (* (`self.SpeedROad`) (`GameplayStatics.GetTimeSeconds`)))) false false))))

(event `Explosion`
  (bind _returnvalue (`self.K2_GetActorLocation`))
  (`/Engine/EditorBlueprintResources/StandardMacros.DoOnce` false
    (:`Completed`
      (set `self.OnMovement?` false)
      (set `self.InitScale` (`SceneComponent.RelativeScale3D` (`self.MainStaticMesh`)))
      (`TimelineComponent.SetPlayRate` (`self.Timeline`) 0.8)
      (bind (_direction _newtrack_0) (`Timeline|Timeline` :!via `PlayFromStart`)
        (:`Update`
          (`SceneComponent.SetRelativeScale3D` (`self.MainStaticMesh`) (`KismetMathLibrary.VLerp` (/ (`self.InitScale`) 2.0) (* (`self.InitScale`) 2.0) _newtrack_0)))
        (:`Finished`
          (`PrimitiveComponent.SetCollisionEnabled` (`self.CapsuleComponent`) "NoCollision")
          (for _array_element (`self.NewMacro`)
            (`PrimitiveComponent.SetSimulatePhysics` _array_element true)
            (`PrimitiveComponent.AddImpulse` _array_element (* (`KismetMathLibrary.RandomUnitVectorInConeInDegrees` (`SceneComponent.GetUpVector` (`self.CapsuleComponent`)) 90.0) 750.0) "None" true))
          (set `self.OnMovement?` false)
          (`GameplayStatics.SpawnEmitterAtLocation` "/Game/Realistic_Starter_VFX_Pack_Vol2/Particles/Explosion/P_Explosion_Big_A.P_Explosion_Big_A" (`SceneComponent.K2_GetComponentLocation` (`self.MainStaticMesh`)))
          (bind _outhits (`KismetSystemLibrary.SphereTraceMulti` _returnvalue (+ _returnvalue (* (`self.GetActorForwardVector`) (`self.DistanceAttack`))) (`self.RadiusAttack`) "TraceTypeQuery1"))
          (for _array_element_2 _outhits
            (`|ExecutionSequence`
              (:`then_0`
                (bind (_bblockinghit _binitialoverlap _time _distance _location _impactpoint _normal _impactnormal _physmat _hitactor _hitcomponent) (`GameplayStatics.BreakHitResult` _array_element_2))
                (bind _asbp_first_person_character (cast `/Game/FirstPerson/Blueprints/BP_FirstPersonCharacter` _hitactor))
                (`/Game/FirstPerson/Blueprints/BP_FirstPersonCharacter.Lose Life` _asbp_first_person_character (`self.Dammage`) false))
              (:`then_1`
                (bind _asbp_ia (cast `/Game/Root/IA/BP_IA` (`ActorComponent.GetOwner` _hitcomponent)))
                (`self.Get Hit` _asbp_ia 25.0 false (0.0 0.0 0.0)))))
          (`self.CallDeath`)
          (`KismetSystemLibrary.Delay` (`self.TimeBeforeDestoy`))
          (`self.K2_DestroyActor`))))))

(fn `AttackBehavior`
  (`self.Explosion`)
  (return))

(fn `CallDeath`
  (`self.Explosion`)
  (`parent.CallDeath`))

(fn `Get Hit`
  (params (HitDamage :type "Float (double-precision)") (isWeakSpot :type Boolean) (LaunchVelocity :type "Vector Structure"))
  (`parent.Get Hit` HitDamage isWeakSpot LaunchVelocity))

(fn `UserConstructionScript`
  (`parent.UserConstructionScript`))