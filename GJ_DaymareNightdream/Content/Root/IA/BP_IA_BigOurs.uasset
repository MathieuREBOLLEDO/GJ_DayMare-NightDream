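; BigOurs AI enemy Blueprint that adds a one-time torso-severing gore effect to the death inherited from its parent, leaving attack behavior unchanged.
; On death it ragdolls the mesh, hides the face and Spine1 bone, adds a skeletal mesh piece at that socket, and spawns blood and VFX_Trip.
; After a one-second delay arms the Decapitation flag, the piece's next hit stamps a single temporary decal.
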(event `self.ReceiveBeginPlay`
  (`parent.ReceiveBeginPlay`))

(event `DecoupeTorse`
  (bind _mesh (`self.Mesh`))
  (bind (_returnvalue_location _returnvalue_rotation) (`KismetMathLibrary.BreakTransform` (`SceneComponent.GetSocketTransform` (`self.Mesh`) "Head" "RTS_World")))
  (bind (_returnvalue_location_2 _returnvalue_rotation_2) (`KismetMathLibrary.BreakTransform` (`SceneComponent.GetSocketTransform` _mesh "Spine1" "RTS_Actor")))
  (`/Engine/EditorBlueprintResources/StandardMacros.DoOnce` false
    (:`Completed`
      (`|ExecutionSequence`
        (:`then_0`
          (`PrimitiveComponent.SetSimulatePhysics` (`self.Mesh`) true)
          (`SceneComponent.SetVisibility` (`self.Face`) false false)
          (bind _returnvalue (`AddComponent|NODE_AddSkeletalMeshComponent-0` :`RelativeTransform` (`KismetMathLibrary.MakeTransform` _returnvalue_location_2 _returnvalue_rotation_2 (75.0 75.0 75.0))))
          (`GameplayStatics.SpawnEmitterAttached` "/Game/Realistic_Starter_VFX_Pack_Vol2/Particles/Blood/P_Blood_Splat_Cone.P_Blood_Splat_Cone" _mesh "Spine1" _returnvalue_location _returnvalue_rotation (7.0 7.0 7.0) "KeepWorldPosition")
          (`SkinnedMeshComponent.HideBoneByName` _mesh "Spine1" "PBO_None")
          (add `PrimitiveComponent.OnComponentHit` _returnvalue (delegate `CustomEvent_2`))
          (`KismetSystemLibrary.Delay` 1.0)
          (set `self.Decapitation?` true))
        (:`then_1`
          (`|SpawnActorFromClass` "/Game/VFXNAGA/trip/VFX_Trip.VFX_Trip_C" (`KismetMathLibrary.MakeTransform` (`SceneComponent.K2_GetComponentLocation` (`self.Scene`))) "Undefined" "MultiplyWithRoot" null null))))))

(event `CustomEvent_2`
  (params (HitComponent :type "PrimitiveComponent Object Reference") (OtherActor :type "Actor Object Reference") (OtherComp :type "PrimitiveComponent Object Reference") (NormalImpulse :type "Vector Structure") (Hit :type "HitResult Structure (by ref)"))
  (if (`self.Decapitation?`)
    (`/Engine/EditorBlueprintResources/StandardMacros.DoOnce` false
      (:`Completed`
        (`GameplayStatics.SpawnDecalAtLocation` "/Game/3Dnchu/Materials/Decal/M_Decal_SoftNnormal.M_Decal_SoftNnormal" (100.0 100.0 100.0) Hit_Location (`KismetMathLibrary.MakeRotFromX` Hit_Normal) 20.0)))))

(fn `AttackBehavior`
  (`parent.AttackBehavior`))

(fn `CallDeath`
  (`parent.CallDeath`)
  (`self.DecoupeTorse`))

(fn `UserConstructionScript`
  (`parent.UserConstructionScript`))