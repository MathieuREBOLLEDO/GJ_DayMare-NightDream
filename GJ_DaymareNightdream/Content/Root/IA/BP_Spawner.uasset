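; BP_Spawner is an enemy spawner that releases a wave of AI enemies at its spawn point and shows a Niagara effect colored by day or night.
; It spawns after a random delay on BeginPlay and on the game instance's day-start event, while night start only recolors the effect.
; Spawn calls itself after random pauses until the count passes NbEnemiesSpawn, picking Ourson, THOMAS or rarer BigOurs by weighted chance.
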(event `self.ReceiveBeginPlay`
  (bind _asmy_gi (`/Game/Root/Utils/Utils.GetGI`))
  (`NiagaraComponent.SetVariableLinearColor` (`self.Niagara`) "Color" (`KismetMathLibrary.SelectColor` (struct :`R` 1000.0 :`G` 8.444965 :`B` 532.09137 :`A` 1.0) (struct :`G` 230.775589 :`B` 1000.0 :`A` 1.0) (`/Game/Root/Utils/MyGI.IsDay?` (`/Game/Root/Utils/Utils.GetGI`))))
  (bind _newfloat (`self.RandomF`))
  (`KismetSystemLibrary.Delay` _newfloat)
  (`self.Spawn`)
  (add `/Game/Root/Utils/MyGI.ED_StartDay` _asmy_gi (delegate `Spawn`))
  (add `/Game/Root/Utils/MyGI.ED_StartNight` _asmy_gi (delegate `StartNight`)))

(event `StartNight`
  (`NiagaraComponent.SetVariableLinearColor` (`self.Niagara`) "Color" (`KismetMathLibrary.SelectColor` (struct :`R` 1000.0 :`G` 0.547 :`B` 37.959576 :`A` 1.0) (struct :`G` 230.775589 :`B` 1000.0 :`A` 1.0) (`/Game/Root/Utils/MyGI.IsDay?` (`/Game/Root/Utils/Utils.GetGI`)))))

(event `Spawn`
  (if (<= (`self.IdEnemies`) (`self.NbEnemiesSpawn`))
    (bind _newfloat (`self.RandomF`))
    (if (< _newfloat 0.85)
      (if (< _newfloat 0.45)
        (set `self.EnemyType` 0)
        (else
          (set `self.EnemyType` 1)))
      (else
        (set `self.EnemyType` 2)))
    (`|SpawnActorFromClass` (select `int` (`self.EnemyType`) :`0` "/Game/Root/IA/BP_IA_Ourson.BP_IA_Ourson_C" :`1` "/Game/Root/IA/BP_IA_THOMAS.BP_IA_THOMAS_C" :`2` "/Game/Root/IA/BP_IA_BigOurs.BP_IA_BigOurs_C" :!type "Actor Class Reference") (`KismetMathLibrary.MakeTransform` (`SceneComponent.K2_GetComponentLocation` (`self.PointToSpawn`))) "AdjustIfPossibleButAlwaysSpawn" "MultiplyWithRoot" null null)
    (`KismetSystemLibrary.Delay` (`KismetMathLibrary.RandomFloatInRange` 0.5 2.5))
    (`/Engine/EditorBlueprintResources/StandardMacros.IncrementInt` (`self.IdEnemies`)
      (:`  `
        (`self.Spawn`)))
    (else
      (set `self.IdEnemies` 0))))

(fn `RandomF`
  (returns (newFloat :type "Float (double-precision)"))
  (return (`KismetMathLibrary.RandomFloat`)))

(fn `UserConstructionScript`)