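; Teddy bear ("Ourson") enemy AI that swaps face material on GameInstance day/night events and reacts to hits with random montages.
; AttackBehavior plays a random montage, flags the blackboard, then after a delay spawns claw VFX and sphere-traces forward to damage the player.
; Death ragdolls then destroys it; weak-spot kills also decapitate by hiding the head bone, adding a mesh component, spawning blood and enabling impact decals.
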(event `self.ReceiveBeginPlay`
  (bind _asmy_gi (`/Game/Root/Utils/Utils.GetGI`))
  (`parent.ReceiveBeginPlay`)
  (add `/Game/Root/Utils/MyGI.ED_StartNight` _asmy_gi (delegate `ChangeFaceNight`))
  (add `/Game/Root/Utils/MyGI.ED_StartDay` _asmy_gi (delegate `ChangeFaceDay`)))

(event `ChangeFaceDay`
  (`PrimitiveComponent.SetMaterial` (`self.Face`) 0 "/Game/Root/IA/Ennemy_01/Scary_Face.Scary_Face"))

(event `ChangeFaceNight`
  (`PrimitiveComponent.SetMaterial` (`self.Face`) 0 "/Game/Root/IA/Ennemy_01/Ennemy_01_Kawai_Face.Ennemy_01_Kawai_Face"))

(event `Decapitation`
  (bind _mesh (`self.Mesh`))
  (bind (_returnvalue_location _returnvalue_rotation) (`KismetMathLibrary.BreakTransform` (`SceneComponent.GetSocketTransform` (`self.Mesh`) "Head" "RTS_World")))
  (bind (_returnvalue_location_2 _returnvalue_rotation_2 _returnvalue_scale) (`KismetMathLibrary.BreakTransform` (`SceneComponent.GetSocketTransform` _mesh "Head" "RTS_Actor")))
  (`/Engine/EditorBlueprintResources/StandardMacros.DoOnce` false
    (:`Completed`
      (`PrimitiveComponent.SetSimulatePhysics` (`self.Mesh`) true)
      (`SceneComponent.SetVisibility` (`self.Face`) false false)
      (bind _returnvalue (`AddComponent|NODE_AddStaticMeshComponent-0` :`RelativeTransform` (`KismetMathLibrary.MakeTransform` _returnvalue_location_2 (struct) _returnvalue_scale)))
      (`|ExecutionSequence`
        (:`then_0`
          (`GameplayStatics.SpawnEmitterAttached` "/Game/Realistic_Starter_VFX_Pack_Vol2/Particles/Blood/P_Blood_Splat_Cone.P_Blood_Splat_Cone" _mesh "Head" _returnvalue_location _returnvalue_rotation (3.0 3.0 3.0) "KeepWorldPosition")
          (`SkinnedMeshComponent.HideBoneByName` _mesh "Head" "PBO_None")
          (add `PrimitiveComponent.OnComponentHit` _returnvalue (delegate `HeadHit`))
          (`KismetSystemLibrary.Delay` 1.0)
          (set `self.Decapitation?` true))
        (:`then_1`
          (`|SpawnActorFromClass` "/Game/VFXNAGA/trip/VFX_Trip.VFX_Trip_C" (`KismetMathLibrary.MakeTransform` (`SceneComponent.K2_GetComponentLocation` (`self.CapsuleComponent`))) "AlwaysSpawn" "MultiplyWithRoot" null (`GameplayStatics.GetPlayerPawn` 0)))))))

(event `HeadHit`
  (params (HitComponent :type "PrimitiveComponent Object Reference") (OtherActor :type "Actor Object Reference") (OtherComp :type "PrimitiveComponent Object Reference") (NormalImpulse :type "Vector Structure") (Hit :type "HitResult Structure (by ref)"))
  (if (`self.Decapitation?`)
    (`/Engine/EditorBlueprintResources/StandardMacros.DoOnce` false
      (:`Completed`
        (`GameplayStatics.SpawnDecalAtLocation` "/Game/3Dnchu/Materials/Decal/M_Decal_SoftNnormal.M_Decal_SoftNnormal" (100.0 100.0 100.0) Hit_Location (`KismetMathLibrary.MakeRotFromX` Hit_Normal) 20.0)))))

(event `self.Mesh.OnComponentHit`
  (params (HitComponent :type "PrimitiveComponent Object Reference") (OtherActor :type "Actor Object Reference") (OtherComp :type "PrimitiveComponent Object Reference") (NormalImpulse :type "Vector Structure") (Hit :type "HitResult Structure (by ref)"))
  (if (`self.Decapitation?`)
    (`/Engine/EditorBlueprintResources/StandardMacros.DoOnce` false
      (:`Completed`
        (`GameplayStatics.SpawnDecalAtLocation` "/Game/Realistic_Starter_VFX_Pack_Vol2/Materials/M_Blood_C_2.M_Blood_C_2" (100.0 100.0 100.0) Hit_Location (`KismetMathLibrary.MakeRotFromX` Hit_Normal) 5.0)
        (`KismetSystemLibrary.PrintString` "Hello")))))

(event `WaitForAttackHit`
  (bind _capsulecomponent (`self.CapsuleComponent`))
  (bind _returnvalue (+ (`self.K2_GetActorLocation`) (`KismetMathLibrary.MakeVector` 0.0 0.0 (`self.OffSetBigOurs`))))
  (bind (_returnvalue_x _returnvalue_y _returnvalue_z) (`KismetMathLibrary.BreakVector` (+ (* (`KismetMathLibrary.GetForwardVector` (`SceneComponent.K2_GetComponentRotation` _capsulecomponent)) 50.0) (`SceneComponent.K2_GetComponentLocation` _capsulecomponent))))
  (`KismetSystemLibrary.Delay` (`self.elapseTimebeforeattackhit`))
  (`NiagaraFunctionLibrary.SpawnSystemAtLocation` "/Game/3Dnchu/Materials/PPInstances/PP_/NS_Claw.NS_Claw" (`KismetMathLibrary.MakeVector` _returnvalue_x _returnvalue_y (+ _returnvalue_z 10.0)) (struct) (0.25 0.25 0.25))
  (bind _outhit (`KismetSystemLibrary.SphereTraceSingle` :`Start` _returnvalue :`End` (+ _returnvalue (* (`self.GetActorForwardVector`) (`self.DistanceAttack`))) :`Radius` (`self.RadiusAttack`) :`TraceChannel` "TraceTypeQuery2" :`DrawDebugType` "ForDuration"))
  (bind (_bblockinghit _binitialoverlap _time _distance _location _impactpoint _normal _impactnormal _physmat _hitactor) (`GameplayStatics.BreakHitResult` _outhit))
  (bind _asbp_first_person_character (cast `/Game/FirstPerson/Blueprints/BP_FirstPersonCharacter` _hitactor)
    (:`then`
      (`/Game/FirstPerson/Blueprints/BP_FirstPersonCharacter.Lose Life` _asbp_first_person_character (`self.Dammage`) false))
    (:`CastFailed`
      (`KismetSystemLibrary.PrintString` (`KismetSystemLibrary.GetDisplayName` _hitactor)))))

(event `DestroyOurson`
  (`PrimitiveComponent.SetSimulatePhysics` (`self.Mesh`) true)
  (`KismetSystemLibrary.Delay` (`self.TimeBeforeDestoy`))
  (`self.K2_DestroyActor`))

(fn `AttackBehavior`
  (set `self.Attack1` (`KismetMathLibrary.RandomBool`))
  (`GameplayStatics.PlaySoundAtLocation` (`self.AttackCue`) (`SceneComponent.K2_GetComponentLocation` (`self.CapsuleComponent`)) (struct) 1.0 1.0 0.0 null null null null)
  (if (`self.Attack1`)
    (`self.PlayAnimMontage` (`self.Anim Montage`))
    (set `self.Attack1` false)
    (else
      (`self.PlayAnimMontage` (`self.AnimMontage2`))
      (set `self.Attack1` true)))
  (`BlackboardComponent.SetValueAsBool` (`AIBlueprintHelperLibrary.GetBlackboard` null) "isAttacking" true)
  (`self.WaitForAttackHit`))

(fn `CallDeath`
  (params (`Thomas?` :type Boolean))
  (`parent.CallDeath` `Thomas?`)
  (`/Engine/EditorBlueprintResources/StandardMacros.DoOnce` false
    (:`Completed`
      (if (`self.isWeakSpot`)
        (`self.Decapitation`)
        (`GameplayStatics.PlaySoundAtLocation` "/Game/Root/Sound_Design/SFX/Enemy1_Ours/E1_Headshot.E1_Headshot" (`SceneComponent.K2_GetComponentLocation` (`self.CapsuleComponent`)) (struct) 1.0 1.0 0.0 null null null null)
        (else
          (`GameplayStatics.PlaySoundAtLocation` (`self.DeathCue`) (`SceneComponent.K2_GetComponentLocation` (`self.CapsuleComponent`)) (struct) 1.0 1.0 0.0 null null null null)))
      (`self.DestroyOurson`))))

(fn `Get Hit`
  (params (HitDamage :type "Float (double-precision)") (isWeakSpot :type Boolean) (LaunchVelocity :type "Vector Structure") (`Thomas?` :type Boolean))
  (`parent.Get Hit` HitDamage isWeakSpot LaunchVelocity `Thomas?`)
  (bind _asbp_ia_big_ours (cast `/Game/Root/IA/BP_IA_BigOurs` self)
    (:`then`
      (`self.PlayAnimMontage` _asbp_ia_big_ours (select `bool` (`KismetMathLibrary.RandomBool`) :`false` "/Game/Root/IA/Ennemy_03/MutantHit1_Montage.MutantHit1_Montage" :`true` "/Game/Root/IA/Ennemy_03/MutantHit2_Montage.MutantHit2_Montage" :!type "AnimMontage Object Reference") (`KismetMathLibrary.RandomFloatInRange` 0.8 1.2) "None"))
    (:`CastFailed`
      (`self.PlayAnimMontage` (select `bool` (`KismetMathLibrary.RandomBool`) :`false` "/Game/Root/IA/Ennemy_01/HappyHit_Montage.HappyHit_Montage" :`true` "/Game/Root/IA/Ennemy_01/HappyHit_Montage.HappyHit_Montage" :!type "AnimMontage Object Reference") (`KismetMathLibrary.RandomFloatInRange` 0.8 1.2)))))

(fn `UserConstructionScript`
  (`parent.UserConstructionScript`))