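; BP_IA is an AI enemy that attacks the first-person player and can be killed.
; AttackBehavior plays a montage, sets the isAttacking Blackboard key and sphere-traces forward with persistent debug drawing, calling LoseLife on the player with 0, leaving Dammage unused.
; GetHit subtracts damage from Life, ignoring the weak-spot flag, and CallDeath sets the isDead key at zero or below.
; The event graph is empty, so these functions rely on external callers.
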(event `self.ReceiveBeginPlay`)

(fn `AttackBehavior`
  (bind _returnvalue (`self.K2_GetActorLocation`))
  (`self.PlayAnimMontage` (`self.Anim Montage`))
  (`BlackboardComponent.SetValueAsBool` (`AIBlueprintHelperLibrary.GetBlackboard` null) "isAttacking" true)
  (bind _outhit (`KismetSystemLibrary.SphereTraceSingle` :`Start` _returnvalue :`End` (+ _returnvalue (* (`self.GetActorForwardVector`) (`self.DistanceAttack`))) :`Radius` (`self.RadiusAttack`) :`TraceChannel` "TraceTypeQuery1" :`DrawDebugType` "Persistent"))
  (bind _asbp_first_person_character (cast `/Game/FirstPerson/Blueprints/BP_FirstPersonCharacter` (`.HitActor` (`GameplayStatics.BreakHitResult` _outhit)))
    (:`then`
      (`/Game/FirstPerson/Blueprints/BP_FirstPersonCharacter.Lose Life` _asbp_first_person_character 0))
    (:`CastFailed`
      _))
  (return))

(fn `CallDeath`
  (`BlackboardComponent.SetValueAsBool` (`AIBlueprintHelperLibrary.GetBlackboard` null) "isDead" true))

(fn `Get Hit`
  (params (HitDamage :type Integer) (isWeakSpot :type Boolean))
  (bind _output_get (set `self.Life` (- (`self.Life`) HitDamage)))
  (if (<= _output_get 0)
    (`self.CallDeath`)))

(fn `UserConstructionScript`)